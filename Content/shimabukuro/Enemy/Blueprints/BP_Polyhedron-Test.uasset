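; Test polyhedron enemy actor that jitters around and can flicker between glowing colors.
; When Animation is set, BeginPlay puts a dynamic M_Lighting instance on the mesh, then loops on a random short delay to randomize its strength and pick one of five colors.
; Tick always applies a random horizontal velocity-change impulse to the mesh; player lookup nodes are present but unused.
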(event EventBeginPlay
  (if (Variables|Default|Getanimation)
    (bind _returnvalue (Rendering|Material|CreateDynamicMaterialInstance (Variables|Default|GetStaticMesh) 0 "/Game/shimabukuro/Stage/Materials/M_Lighting.M_Lighting" "None" :!class /Script/Engine.PrimitiveComponent))
    (Variables|Default|SetDynamicMaterialInstanceA _returnvalue)
    (Rendering|Material|SetMaterial (Variables|Default|GetStaticMesh) 0 (Variables|Default|GetDynamicMaterialInstanceA))
    (Utilities|FlowControl|Delay (Math|Random|RandomFloatinRange 0.2 1.0) :!label _label)
    (Rendering|Material|SetScalarParameterValue (Variables|Default|GetDynamicMaterialInstanceA) "strength" (Math|Random|RandomFloatinRange 5.0 1e+01) :!class /Script/Engine.MaterialInstanceDynamic)
    (switch int (Math|Random|RandomInteger 5)
      (:Default
        (Rendering|Material|SetVectorParameterValue (Variables|Default|GetDynamicMaterialInstanceA) "color" "(R=1.000000,G=1.000000,B=1.000000,A=1.000000)" :!class /Script/Engine.MaterialInstanceDynamic)
        (goto _label))
      (:0
        (Rendering|Material|SetVectorParameterValue (Variables|Default|GetDynamicMaterialInstanceA) "color" "(R=0.000000,G=0.351533,B=1.000000,A=1.000000)" :!class /Script/Engine.MaterialInstanceDynamic)
        (goto _label))
      (:1
        (Rendering|Material|SetVectorParameterValue (Variables|Default|GetDynamicMaterialInstanceA) "color" "(R=0.012983,G=1.000000,B=0.000000,A=1.000000)" :!class /Script/Engine.MaterialInstanceDynamic)
        (goto _label))
      (:2
        (Rendering|Material|SetVectorParameterValue (Variables|Default|GetDynamicMaterialInstanceA) "color" "(R=1.000000,G=0.309469,B=0.000000,A=1.000000)" :!class /Script/Engine.MaterialInstanceDynamic)
        (goto _label))
      (:3
        (Rendering|Material|SetVectorParameterValue (Variables|Default|GetDynamicMaterialInstanceA) "color" "(R=1.000000,G=0.000000,B=0.313989,A=1.000000)" :!class /Script/Engine.MaterialInstanceDynamic)
        (goto _label)))))

(event EventTick
  (params (DeltaSeconds :type Float%20%28single-precision%29))
  (Physics|AddImpulse (Variables|Default|GetStaticMesh) (* (Math|Random|RandomUnitVector) "100.000000,100.000000,0.000000") "None" true))

(fn ConstructionScript)